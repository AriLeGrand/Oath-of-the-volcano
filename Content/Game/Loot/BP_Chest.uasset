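; BP_Chest is a one-time loot chest that gives the overlapping player a random DT_Items item with a rolled rarity.
; Rarity uses a GameMode-held pity bonus that shifts rolls toward rarer tiers, grows on lowest-tier results and resets on the top two.
; The item goes to the player and appears as a rotating mesh while a Timeline opens the lid, then disappears.
; The chest destroys itself on the GameMode's cycle reset.
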(event OnComponentBeginOverlap(Box)
  (params (OverlappedComponent :type Primitive%20Component%20Object%20Reference) (OtherActor :type Actor%20Object%20Reference) (OtherComp :type Primitive%20Component%20Object%20Reference) (OtherBodyIndex :type Integer) (bFromSweep :type Boolean) (SweepResult :type Hit%20Result%20Structure%20%28by%20ref%29))
  (bind _floatingitem (Variables|Default|GetFloatingItem))
  (bind _gamemode (Variables|Default|GetgameMode))
  (bind _asplayer_character (Utilities|Casting|CastToPlayerCharacter OtherActor))
  (Variables|Default|SetRefJoueur _asplayer_character)
  ;[0.15 0.15 0.15 0.5] Random Chest Loot System
  (Utilities|FlowControl|DoOnce false
    (:Completed
      (bind _outrownames (DataTable|GetDataTableRowNames "/Game/Game/Loot/DT_Items.DT_Items"))
      (bind _returnvalue (Utilities|GetDataTableRow "/Game/Game/Loot/DT_Items.DT_Items" (Utilities|Array|Get(acopy) _outrownames (Math|Random|RandomIntegerinRange 0 (- (Utilities|Array|Length _outrownames) 1))))
        (:then
          ;[0.15 0.15 0.15 0.5] Rarity + Pity System
          (bind _output_get (Variables|Default|SetRollValue (- (Math|Random|RandomFloatinRange 0.0 1e+02) (Variables|/Game/Game/MainGameMode.MainGameMode_C|GetPityBonus (Variables|Default|GetgameMode)))))
          (if (<= _output_get 3.0)
            (Variables|Default|SetChosenRarity "NewEnumerator3")
            (Variables|/Game/Game/MainGameMode.MainGameMode_C|SetPityBonus (Variables|Default|GetgameMode) 0.0 :!label _label)
            (elif (<= _output_get 15.0)
              (Variables|Default|SetChosenRarity "NewEnumerator2")
              (goto _label)
              (elif (<= _output_get 35.0)
                (Variables|Default|SetChosenRarity "NewEnumerator1")
                (else
                  (Variables|Default|SetChosenRarity "NewEnumerator0")
                  (Variables|/Game/Game/MainGameMode.MainGameMode_C|SetPityBonus _gamemode (+ (Variables|/Game/Game/MainGameMode.MainGameMode_C|GetPityBonus _gamemode) 2.0))))))
          (Default|ReceiveItem (Variables|Default|GetRefJoueur) (.itemName (Utilities|Struct|BreakST_Item _returnvalue)) (Variables|Default|GetChosenRarity))
          (Components|StaticMesh|SetStaticMesh _floatingitem (.ItemMesh (Utilities|Struct|BreakST_Item _returnvalue)))
          (Development|SetHiddeninGame _floatingitem false false)
          (bind _alpha (Timeline|Timeline Play)
            (:Update
              (Transformation|SetRelativeLocation (Variables|Default|GetChestLid) (Math|Vector|Lerp(Vector) "2.000000,0.000000,66.500000" "-23.218477,-36.277106,66.500000" _alpha) false false)
              (Transformation|SetRelativeRotation (Variables|Default|GetChestLid) (Math|Rotator|Lerp(Rotator) "0, 0, 0" "0.000000,50.000000,0.000000" _alpha) false false))
            (:Finished
              (Utilities|FlowControl|Delay 3.0)
              (Components|DestroyComponent (Variables|Default|GetFloatingItem)))))))))

(event EventOnCycleReset
  (Actor|DestroyActor))

(event EventEndPlay
  (params (EndPlayReason :type EEndPlayReason%20Enum :default "Destroyed"))
  (EventDispatchers|UnbindEventfromOnCycleReset (Variables|Default|GetgameMode) (delegate EventOnCycleReset)))

(event EventBeginPlay
  (Utilities|GetMainGameMode (Variables|Default|GetgameMode))
  (EventDispatchers|BindEventtoOnCycleReset (Variables|Default|GetgameMode) (delegate EventOnCycleReset))
  (Components|Movement|SetUpdatedComponent (Variables|Default|GetRotatingMovement) (Variables|Default|GetFloatingItem)))

(fn ConstructionScript)