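; BP_Crab is an AI enemy that repeatedly damages the player on contact and can be killed.
; A looping timer runs while the player's hitbox overlaps its box.
; Hits subtract health and briefly flash a dynamic material, destroying the crab at zero health.
; It binds to GameInstance pause, unpause, reset and player-spawn events, with helpers to halt or restart AI and movement, restore its starting transform and fetch the player.
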(event OnComponentBeginOverlap(Box)
  (params (OverlappedComponent :type Primitive%20Component%20Object%20Reference) (OtherActor :type Actor%20Object%20Reference) (OtherComp :type Primitive%20Component%20Object%20Reference) (OtherBodyIndex :type Integer) (bFromSweep :type Boolean) (SweepResult :type Hit%20Result%20Structure%20%28by%20ref%29))
  (if (Components|ComponentHasTag OtherComp "PlayerHitbox")
    (bind _returnvalue (Utilities|Time|SetTimerbyEvent (EventDispatchers|CreateEvent :!event TickPlayerforDamage) (Variables|Default|GetdamageTickSpeed) true))
    (Variables|Default|SettickPlayerForDamageTimer _returnvalue)))

(event OnComponentEndOverlap(Box)
  (params (OverlappedComponent :type Primitive%20Component%20Object%20Reference) (OtherActor :type Actor%20Object%20Reference) (OtherComp :type Primitive%20Component%20Object%20Reference) (OtherBodyIndex :type Integer))
  (if (Components|ComponentHasTag OtherComp "PlayerHitbox")
    (Utilities|Time|ClearandInvalidateTimerbyHandle (Variables|Default|GettickPlayerForDamageTimer))))

(event EventOnHit
  (params (damage :type Float%20%28double-precision%29) (direction :type Vector :default "0, 0, 0"))
  (Utilities|FlowControl|Sequence
    (:then_0
      ;[0.15 0.15 0.15 0.5] Take hit
      (CallFunction|SubtractHealth damage))
    (:then_1
      ;[0.15 0.15 0.15 0.5] HitMarker
      (Rendering|Material|SetScalarParameterValue (Variables|Default|GetDynamicCrabMaterial) "Intensity" 0.5 :!class /Script/Engine.MaterialInstanceDynamic)
      (Utilities|FlowControl|Delay 0.1)
      (Rendering|Material|SetScalarParameterValue (Variables|Default|GetDynamicCrabMaterial) "Intensity" 0.0 :!class /Script/Engine.MaterialInstanceDynamic))
    (:then_2
      ;[0.15 0.15 0.15 0.5] Death + VFX
      (if (<= (Variables|Default|GetHealth) 0.0)
        (Rendering|SetVisibility (Variables|Components|GetCrabmodel) false false)
        (Actor|DestroyActor)))))

(event EventBeginPlay
  (Variables|Default|SetinitialTransformData (Transformation|GetActorTransform))
  (Utilities|GetMainGameInstance (Variables|Default|GetgameInstance))
  (EventDispatchers|BindEventtoOnGamePaused (Variables|Default|GetgameInstance) (EventDispatchers|CreateEvent :!event DisableAI))
  (EventDispatchers|BindEventtoOnGameUnpaused (Variables|Default|GetgameInstance) (EventDispatchers|CreateEvent :!event EnableAI))
  (EventDispatchers|BindEventtoOnGameReset (Variables|Default|GetgameInstance) (EventDispatchers|CreateEvent :!event Reset))
  (EventDispatchers|BindEventtoOnPlayerSpawned (Variables|Default|GetgameInstance) (EventDispatchers|CreateEvent :!event GetPlayer))
  (Variables|Default|SetinitialSpeed (Class|MovementComponent|GetMaxSpeed (Variables|Character|GetCharacterMovement)))
  (Variables|Default|SetBrain%20Component (Variables|/Script/AIModule.AIController|GetBrainComponent (AI|GetAIController self)))
  (bind _returnvalue (Rendering|Material|CreateDynamicMaterialInstance (Variables|Components|GetCrabmodel) 0 "/Game/Art/Character/Global/MasterLibrary/MI_Crab_01.MI_Crab_01" "None" :!class /Script/Engine.PrimitiveComponent))
  (Variables|Default|SetDynamicCrabMaterial _returnvalue))

(event EventEndPlay
  (params (EndPlayReason :type EEndPlayReason%20Enum :default "Destroyed"))
  (EventDispatchers|UnbindEventfromOnGamePaused (Variables|Default|GetgameInstance) (EventDispatchers|CreateEvent :!event DisableAI))
  (EventDispatchers|UnbindEventfromOnGameUnpaused (Variables|Default|GetgameInstance) (EventDispatchers|CreateEvent :!event EnableAI))
  (EventDispatchers|UnbindEventfromOnGameReset (Variables|Default|GetgameInstance) (EventDispatchers|CreateEvent :!event Reset))
  (EventDispatchers|UnbindEventfromOnPlayerSpawned (Variables|Default|GetgameInstance) (EventDispatchers|CreateEvent :!event GetPlayer)))

(fn ConstructionScript)

(fn SubtractHealth
  (params (Damage :type Float%20%28double-precision%29))
  (Variables|Default|SetHealth (- (Variables|Default|GetHealth) Damage)))

(fn EnableAI
  (Class|BrainComponent|RestartLogic (Variables|Default|GetBrain%20Component))
  (Variables|/Script/Engine.CharacterMovementComponent|SetMaxWalkSpeed (Variables|Character|GetCharacterMovement) (Variables|Default|GetinitialSpeed)))

(fn DisableAI
  (AI|Logic|StopLogic (Variables|Default|GetBrain%20Component) "")
  (Variables|/Script/Engine.CharacterMovementComponent|SetMaxWalkSpeed (Variables|Character|GetCharacterMovement) 0.0))

(fn GetPlayer
  (Utilities|GetPlayer (Variables|Default|Getplayer)))

(fn TickPlayerforDamage
  (Default|TakeDamage (Variables|Default|Getplayer) (Variables|Default|GetDamage)))

(fn Reset
  (Transformation|SetActorTransform (Variables|Default|GetinitialTransformData)))

(fn IsRelevanttoComboSystem
  (return true))