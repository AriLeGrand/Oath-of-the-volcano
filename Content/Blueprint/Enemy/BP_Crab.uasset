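; Crab enemy actor that takes damage and destroys itself when its health runs out.
; OnHit passes Damage to SubscractHP, which subtracts it from Health.
; At zero or below, it hides the crab model, shows a Plane as a placeholder explosion effect, then destroys the actor after a short delay.
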(event EventOnHit
  (params (damage :type Float%20%28double-precision%29) (direction :type Vector :default "0, 0, 0"))
  ;[0.15 0.15 0.15 0.5] Death
  (CallFunction|SubscractHP damage)
  (if (<= (Variables|Default|GetHealth) 0.0)
    ;;[0.15 0.15 0.15 0.5] Explosion VFX Placeholder
    (Rendering|SetVisibility (Variables|Components|GetCrabmodel) false false)
    (Rendering|SetVisibility (Variables|Components|GetPlane) true false)
    (Utilities|FlowControl|Delay 0.2)
    (Actor|DestroyActor)))

(fn ConstructionScript)

(fn SubscractHP
  (params (Damage :type Float%20%28double-precision%29))
  (Variables|Default|SetHealth (- (Variables|Default|GetHealth) Damage)))