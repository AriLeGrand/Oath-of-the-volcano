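; BP_ItemManager populates the level's item placeholders with random items and can shuffle their positions.
; On BeginPlay it gathers every BP_ItemPlaceHolder, spawns a random ItemTypeList entry at each one's transform, and records it on the placeholder and in a list.
; ShuffleItems randomizes that list, then teleports each item to the next one's location, wrapping around, without updating the placeholders' CurrentItem references.
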(event EventBeginPlay
  (bind _numberofplaceholder (CallFunction|GetNumberOfItemPlaceolder))
  (Variables|Default|SetNumberOfItemPlaceHolder _numberofplaceholder)
  (CallFunction|CreateItems))

(fn GetNumberOfItemPlaceolder
  (bind _outactors (Actor|GetAllActorsOfClass "/Game/Items/BP_ItemPlaceHolder.BP_ItemPlaceHolder_C"))
  (bind _output_get (Variables|Default|SetPlaceHolderList _outactors))
  (return (Utilities|Array|Length _output_get)))

(fn CreateItems
  (for _index (range 0 (Variables|Default|GetNumberOfItemPlaceHolder))
    (Utilities|IsValid (Utilities|Array|Get(acopy) (Variables|Default|GetPlaceHolderList) _index)
      (:Is%20Valid
        (bind _returnvalue (Game|SpawnActorfromClass (.OutItem (Utilities|Array|Random (Variables|Default|GetItemTypeList))) (Transformation|GetActorTransform (Utilities|Array|Get(acopy) (Variables|Default|GetPlaceHolderList) _index)) "Undefined" "MultiplyWithRoot" 0 0))
        (bind _output_get (Variables|/Game/Items/BP_ItemPlaceHolder.BP_ItemPlaceHolder_C|SetCurrentItem (Utilities|Array|Get(acopy) (Variables|Default|GetPlaceHolderList) _index) _returnvalue))
        (Utilities|Array|Add (Variables|Default|GetItemInPlaceHolderList) _output_get))
      (:Is%20Not%20Valid
        (return)))))

(fn ShuffleItems
  (bind _iteminplaceholderlist (Variables|Default|GetItemInPlaceHolderList))
  (bind _iteminplaceholderlist_2 (Variables|Default|GetItemInPlaceHolderList))
  (Utilities|Array|Shuffle _iteminplaceholderlist)
  (LocalVariables|SetPrevious%20location (Transformation|GetActorLocation (Utilities|Array|Get(acopy) _iteminplaceholderlist)))
  (for (_array_element _array_index) (Variables|Default|GetItemInPlaceHolderList)
    (if (Utilities|Array|IsValidIndex _iteminplaceholderlist_2 (+ _array_index 1))
      (LocalVariables|SetNewLocation (Transformation|GetActorLocation (Utilities|Array|Get(acopy) _iteminplaceholderlist_2 (+ _array_index 1))))
      (else
        (LocalVariables|SetNewLocation (LocalVariables|GetPrevious%20location))))
    (Transformation|SetActorLocation _array_element (LocalVariables|GetNewLocation) false true)))