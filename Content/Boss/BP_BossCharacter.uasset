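; BP_BossCharacter is the boss enemy, with health, a chase speed, and rock-launch and shockwave attacks.
; On BeginPlay it writes half of max health to its BP_BossControler blackboard, and hits update the current health there and clear IsAlive on overkill.
; Attacks reuse one cached actor each, spawning it only when missing: the rock is repositioned and launched by impulse, and the shockwave moves to the boss only once finished.
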(event EventOnHit
  (params (damage :type Float%20%28double-precision%29) (direction :type Vector :default "0, 0, 0"))
  ;[0.7313 0.3698 1 0.5] When the boss is hit it will take damage
  (if (Variables|Default|GetIsAlive)
    (CallFunction|TakeDamage damage)
    (Development|PrintString (Utilities|String|ToString(Float) (Variables|Default|GetCurrentHealth)))))

(event EventBeginPlay
  ;[1 0.5035 0.5 0.5] Sets a blackboard value
  (bind _asbp_boss_controler (Utilities|Casting|CastToBP_BossControler (Pawn|GetController)))
  (bind _output_get (Variables|Default|SetBossControler _asbp_boss_controler))
  (AI|Components|Blackboard|SetValueasFloat (Variables|/Script/AIModule.AIController|GetBlackboard _output_get) (Variables|Default|GetHalfedHealth) (/ (Variables|Default|GetMaxHealth) 2.0)))

(fn ConstructionScript)

(fn UpdateWalkSpeed
  (params (NewWalkSpeed :type Float%20%28double-precision%29))
  (Variables|/Script/Engine.CharacterMovementComponent|SetMaxWalkSpeed (Variables|Character|GetCharacterMovement) NewWalkSpeed))

(fn TakeDamage
  (params (Damage :type Float%20%28double-precision%29))
  ;[1 0.3906 0.6015 0.5] Decrease the enemy health
  (Variables|Default|SetwillDie (> Damage (Variables|Default|GetCurrentHealth)))
  (bind _output_get (Variables|Default|SetCurrentHealth (Math|Float|Clamp(Float) (- (Variables|Default|GetCurrentHealth) Damage) 0.0 (Variables|Default|GetMaxHealth))))
  (AI|Components|Blackboard|SetValueasFloat (Variables|/Script/AIModule.AIController|GetBlackboard (Variables|Default|GetBossControler)) (Variables|Default|GetBB%20CurrentHealth) _output_get)
  (Variables|Default|SetIsAlive (not (Variables|Default|GetWillDie)))
  (return))

(fn ChasePlayer
  (CallFunction|UpdateWalkSpeed (Variables|Default|GetChaseSpeed))
  (return true))

(fn IsRelevanttoComboSystem
  (return true))

(fn RockLaunch
  (bind _rock_ref (Variables|Default|GetRock%20Ref)
    (:then
      (Transformation|SetActorLocation _rock_ref (Transformation|GetActorLocation) true true))
    (:else
      (bind _returnvalue (Game|SpawnActorfromClass "/Game/Boss/BP_Rock.BP_Rock_C" (Transformation|GetActorTransform) "Undefined" "MultiplyWithRoot" 0 0))
      (bind _output_get (Variables|Default|SetRock%20Ref _returnvalue))
      ;[1 0.5335 0.09375 0.5] Lauch rock
      (Collision|IgnoreActorwhenMoving (Variables|/Game/Boss/BP_Rock.BP_Rock_C|GetStaticMesh _output_get) 0 true)))
  (Physics|AddImpulse (Variables|/Game/Boss/BP_Rock.BP_Rock_C|GetStaticMesh (Variables|Default|GetRock%20Ref)) (* (+ (Transformation|GetActorForwardVector) "0.500000,0.000000,0.500000") 3e+04) "None" false)
  (return true))

(fn ShockWave
  (bind _returnvalue (Transformation|GetActorTransform))
  (bind _shockwaveref (Variables|Default|GetShockWaveRef)
    (:then
      (if (Variables|/Game/Boss/BP_ShockWave.BP_ShockWave_C|GetIsFinshed _shockwaveref)
        (Transformation|SetActorTransform _shockwaveref _returnvalue)
        (Collision|IgnoreActorwhenMoving (Variables|Default|GetBox) (stale _output_get) true :!label _label)
        (return true)))
    (:else
      ;[0.9278 0.6037 0.974 0.5] If empty instatiate actor and set the reference
      (bind _returnvalue_2 (Game|SpawnActorfromClass "/Game/Boss/BP_ShockWave.BP_ShockWave_C" _returnvalue "Undefined" "MultiplyWithRoot" 0 0))
      (bind _output_get (Variables|Default|SetShockWaveRef _returnvalue_2))
      (goto _label))))