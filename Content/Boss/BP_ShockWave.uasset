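; BP_ShockWave is a boss shockwave actor that expands from spawn and knocks the player back.
; A Timeline started on BeginPlay scales the root uniformly, and the actor destroys itself when it finishes.
; Overlapping the cached player character applies a large impulse along fixed world +X and upward, independent of the wave's position or facing.
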(event Custom|IsShockWaveAtMaxSize
  (if (Variables|Default|GetIsFinshed)
    (Actor|DestroyActor)))

(event EventBeginPlay
  (bind _asplayer_character (Utilities|Casting|CastToPlayerCharacter (Game|Player|GetPlayerPawn 0)))
  (Variables|Default|Setplayer _asplayer_character)
  (bind _scalefactor (Timeline|Timeline Play)
    (:Update
      (Transformation|SetWorldScale3D (Variables|Default|GetDefaultSceneRoot) (* _scalefactor "1.000000,1.000000,1.000000")))
    (:Finished
      (Variables|Default|SetIsFinshed true)
      (CallFunction|IsShockWaveatMaxSize))))

(event Collision|EventActorBeginOverlap
  (params (OtherActor :type Actor%20Object%20Reference))
  (if (== OtherActor (Variables|Default|Getplayer))
    (Physics|AddImpulse (Variables|/Script/Engine.Character|GetCharacterMovement (Variables|Default|Getplayer)) "600000.000000,0.000000,60000.000000" false)))

(fn ConstructionScript)