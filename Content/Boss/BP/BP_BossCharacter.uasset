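; Boss character with a Moai-head material that takes hits and provides chase, rock launch and shockwave actions.
; Health is mirrored to the AI controller's Blackboard along with a half-health threshold, and hits briefly raise a dynamic material's intensity as a hit marker.
; Rock launches spawn and impulse a new rock, while the shockwave reuses one cached actor, repositioning it once finished.
; It also reports itself as relevant to the combo system.
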(event EventOnHit
  (params (damage :type Float%20%28double-precision%29) (direction :type Vector :default "0, 0, 0"))
  ;[0.7313 0.3698 1 0.5] When the boss is hit it will take damage
  (if (Variables|Health|GetIsAlive)
    (Utilities|FlowControl|Sequence
      (:then_0
        (CallFunction|TakeDamage damage))
      (:then_1
        ;;[0.15 0.15 0.15 0.5] Hit marker
        (Rendering|Material|SetScalarParameterValue (Variables|HitMarker|GetDynamic%20Moai%20Material) "Intensity" 0.2 :!class /Script/Engine.MaterialInstanceDynamic)
        (Utilities|FlowControl|Delay 0.2)
        (Rendering|Material|SetScalarParameterValue (Variables|HitMarker|GetDynamic%20Moai%20Material) "Intensity" 0.0 :!class /Script/Engine.MaterialInstanceDynamic)))))

(event EventBeginPlay
  ;[1 0.5035 0.5 0.5] Sets a blackboard value
  (bind _asbp_boss_controler (Utilities|Casting|CastToBP_BossControler (Pawn|GetController)))
  (bind _output_get (Variables|Default|SetBossControler _asbp_boss_controler))
  (AI|Components|Blackboard|SetValueasFloat (Variables|/Script/AIModule.AIController|GetBlackboard _output_get) (Variables|Health|Blackboard|GetHalfedHealth) (/ (Variables|Health|GetMaxHealth) 2.0))
  (bind _returnvalue (Rendering|Material|CreateDynamicMaterialInstance (Variables|Default|GetStaticMesh) 0 "/Game/Art/Character/Global/MasterLibrary/MI_MoaiHead_03.MI_MoaiHead_03" "None" :!class /Script/Engine.PrimitiveComponent))
  (Variables|HitMarker|SetDynamic%20Moai%20Material _returnvalue))

(fn ConstructionScript)

(fn UpdateWalkSpeed
  (params (NewWalkSpeed :type Float%20%28double-precision%29))
  (Variables|/Script/Engine.CharacterMovementComponent|SetMaxWalkSpeed (Variables|Character|GetCharacterMovement) NewWalkSpeed))

(fn TakeDamage
  (params (Damage :type Float%20%28double-precision%29))
  ;[1 0.3906 0.6015 0.5] Decrease the enemy health
  (Variables|Default|SetwillDie (> Damage (Variables|Health|GetCurrentHealth)))
  (bind _output_get (Variables|Health|SetCurrentHealth (Math|Float|Clamp(Float) (- (Variables|Health|GetCurrentHealth) Damage) 0.0 (Variables|Health|GetMaxHealth))))
  (AI|Components|Blackboard|SetValueasFloat (Variables|/Script/AIModule.AIController|GetBlackboard (Variables|Default|GetBossControler)) (Variables|Health|Blackboard|GetBB%20CurrentHealth) _output_get)
  (Variables|Health|SetIsAlive (not (Variables|Health|GetWillDie)))
  (return))

(fn ChasePlayer
  ;[1 0.276 0.5268 0.5] Chasing the player
  (CallFunction|UpdateWalkSpeed (Variables|Movement|GetChaseSpeed))
  (return true))

(fn IsRelevanttoComboSystem
  (return true))

(fn RockLaunch
  ;[1 0.276 0.5268 0.5] Check for empty reference
  ;[0.1832 0.3308 0.9635 0.5] If  reference isn't empty set the new location to the  boss's
  (bind _returnvalue (Game|SpawnActorfromClass "/Game/Boss/BP/Attacks/BP_Rock.BP_Rock_C" (Transformation|GetActorTransform) "Undefined" "MultiplyWithRoot" 0 0))
  ;[1 0.5335 0.09375 0.5] Lauch rock
  (Physics|AddImpulse (Variables|/Game/Boss/BP/Attacks/BP_Rock.BP_Rock_C|GetStaticMesh _returnvalue) (* (+ (Transformation|GetActorForwardVector) "0.500000,0.000000,0.500000") (Variables|Attacks|GetRockLaunchForce)) "None" false)
  (return true))

(fn ShockWave
  (bind _returnvalue (Transformation|GetActorTransform))
  (bind _shockwaveref (Variables|Attacks|GetShockWaveRef)
    (:then
      (if (Variables|/Game/Boss/BP/Attacks/BP_ShockWave.BP_ShockWave_C|GetIsFinshed _shockwaveref)
        (Transformation|SetActorTransform _shockwaveref _returnvalue)
        (return true)))
    (:else
      ;[0.9278 0.6037 0.974 0.5] If empty instatiate actor and set the reference
      (bind _returnvalue_2 (Game|SpawnActorfromClass "/Game/Boss/BP/Attacks/BP_ShockWave.BP_ShockWave_C" _returnvalue "Undefined" "MultiplyWithRoot" 0 0))
      (Variables|Attacks|SetShockWaveRef _returnvalue_2)
      (return true))))