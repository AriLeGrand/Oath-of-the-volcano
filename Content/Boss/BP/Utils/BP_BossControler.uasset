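; BP_BossControler is the boss's AI controller, which runs BT_Boss on possess and tracks whether the boss can see the player.
; AI perception writes a sensed Player-tagged actor to the blackboard as PlayerCharacter and sets HasPlayerInSight.
; Any other perception update starts a LineOfSightTimer-long memory timer, which clears both keys on expiry and is cancelled when the player is sensed again.
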(event OnTargetPerceptionUpdated(AIPerception)
  (params (Actor :type Actor%20Object%20Reference) (Stimulus :type AI%20Stimulus%20Structure))
  (bind _blackboard (Variables|Default|GetBlackboard))
  ;[0.9278 0.6037 0.974 0.5] Check if the player has been seen
  ;;[1 0.6273 0.276 0.5] Sets the black board values
  (if (and (Actor|ActorHasTag Actor "Player") (.bSuccessfullySensed (Utilities|Struct|BreakAIStimulus Stimulus)))
    (Utilities|Time|ClearandInvalidateTimerbyHandle (Variables|Default|GetEnemyTimer))
    (AI|Components|Blackboard|SetValueasBool _blackboard (Variables|Default|GetHasPlayerInSight) true)
    (AI|Components|Blackboard|SetValueasObject _blackboard (Variables|Default|GetPlayerCharacter) Actor)
    (else
      ;;[1 0.1667 0.2403 0.5] How long does the enemy remembers the player
      (bind _returnvalue (Utilities|Time|SetTimerbyEvent (delegate Custom|StartEnemyTimer) (Variables|Default|GetLineOfSightTimer)))
      (Variables|Default|SetEnemyTimer _returnvalue))))

(event Custom|StartEnemyTimer
  (bind _blackboard (Variables|Default|GetBlackboard))
  ;[0.9278 0.6037 0.974 0.5] Check if the player has been seen
  ;;[1 0.1667 0.2403 0.5] How long does the enemy remembers the player
  (AI|Components|Blackboard|SetValueasBool _blackboard (Variables|Default|GetHasPlayerInSight) false)
  (AI|Components|Blackboard|SetValueasObject _blackboard (Variables|Default|GetPlayerCharacter) 0))

(event EventPossess
  (params (PossessedPawn :type Pawn%20Object%20Reference))
  ;[0.9278 0.6037 0.974 0.5] Check if the player has been seen
  (AI|RunBehaviorTree "/Game/Boss/BT_Boss.BT_Boss"))

(fn ConstructionScript)