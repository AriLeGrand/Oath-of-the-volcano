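; BP_BossHead is a boss attack actor: a homing head projectile that damages and launches the player.
; On BeginPlay it sets the player's root component as its ProjectileMovement homing target and caches the PlayerCharacter reference.
; Overlapping the player applies a fixed world-space impulse along +X and +Z, regardless of approach direction, then calls TakeDamage with HeadDammage.
; The graph never destroys the projectile after a hit.
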(event EventBeginPlay
  (Variables|/Script/Engine.ProjectileMovementComponent|SetHomingTargetComponent (Variables|Default|GetProjectileMovement) (Variables|/Script/Engine.Actor|GetRootComponent (Game|GetPlayerCharacter 0)))
  (bind _asplayer_character (Utilities|Casting|CastToPlayerCharacter (Game|GetPlayerCharacter 0)))
  (Variables|Default|SetPayerRef _asplayer_character))

(event Collision|EventActorBeginOverlap
  (params (OtherActor :type Actor%20Object%20Reference))
  (bind _payerref (Variables|Default|GetPayerRef))
  (if (== OtherActor _payerref)
    (Physics|AddImpulse (Variables|/Script/Engine.Character|GetCharacterMovement _payerref) "10000.000000,0.000000,10000.000000" false)
    (Default|TakeDamage _payerref (Variables|Default|GetHeadDammage))))

(fn ConstructionScript)