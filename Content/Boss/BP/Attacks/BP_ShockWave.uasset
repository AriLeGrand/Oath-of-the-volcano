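; Boss shock wave attack actor that expands on spawn and knocks the player back on contact.
; On BeginPlay it gets the player reference and plays a timeline that uniformly scales the Sphere component, then destroys the actor when the timeline finishes.
; When the sphere begins overlapping the player, it adds a mass-dependent CharacterMovement impulse of ImpulseStrength, directed away from the wave's center.
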(event OnComponentBeginOverlap(Sphere)
  (params (OverlappedComponent :type Primitive%20Component%20Object%20Reference) (OtherActor :type Actor%20Object%20Reference) (OtherComp :type Primitive%20Component%20Object%20Reference) (OtherBodyIndex :type Integer) (bFromSweep :type Boolean) (SweepResult :type Hit%20Result%20Structure%20%28by%20ref%29))
  (bind _player (Variables|Default|Getplayer))
  ;[0.5938 0.7167 1 0.5] When the player touches the shockwave it bounces back
  (if (== OtherActor (Variables|Default|Getplayer))
    (Physics|AddImpulse (Variables|/Script/Engine.Character|GetCharacterMovement _player) (* (Variables|Default|GetimpulseStrength) (Math|Vector|Normalize (- (Transformation|GetActorLocation _player) (Transformation|GetActorLocation)))) false)))

(event Custom|IsShockWaveAtMaxSize
  ;[1 0.1443 0] When at max size delete the shock wave
  (if (Variables|Default|GetIsFinshed)
    (Actor|DestroyActor)))

(event EventBeginPlay
  ;[0.7313 0.3698 1 0.5] Scales up the actor when it spawn
  (Utilities|GetPlayer (Variables|Default|Getplayer))
  (bind _scalefactor (Timeline|Timeline Play)
    (:Update
      (Transformation|SetWorldScale3D (Variables|Default|GetSphere) (* _scalefactor "1.000000,1.000000,1.000000")))
    (:Finished
      (Variables|Default|SetIsFinshed true)
      (CallFunction|IsShockWaveatMaxSize))))

(fn ConstructionScript)